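; Test character with a "jacking" mode that switches to an overhead camera for picking an Enemy with the mouse.
; P plays a timeline that pitches control rotation downward and extends the spring arm, then shows the cursor and enables jacking.
; Left-clicking an Enemy under the cursor plays a second timeline that restores the closer view, hides the cursor, exits the mode and calls that enemy's Pulse.
; Debug strings print on each click while jacking.
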(event `Key|P`
  (params (Key :type "Key Structure"))
  (bind _springarmcomp (`self.SpringArmComp`))
  (:`Pressed`
    (bind (_direction _newtrack_0) (`Timeline|Timeline` :!via `PlayFromStart`)
      (:`Update`
        (bind (_returnvalue_x _returnvalue_y _returnvalue_z) (`KismetMathLibrary.BreakVector` (`KismetMathLibrary.VInterpTo` (0.0 0.0 0.0) (0.0 -90.0 0.0) _newtrack_0 1.0)))
        (`Controller.SetControlRotation` (`self.GetController`) (`KismetMathLibrary.MakeRotator` _returnvalue_x _returnvalue_y _returnvalue_z))
        (set `SpringArmComponent.TargetArmLength` (`|EaseFunction` "Linear" _newtrack_0 (`SpringArmComponent.TargetArmLength` _springarmcomp) 2000.0) _springarmcomp))
      (:`Finished`
        (bind _asplayer_controller (cast `PlayerController` (`self.GetController`)))
        (set `PlayerController.bShowMouseCursor` true _asplayer_controller)
        (set `self.jacking` true)))))

(event `Key|LeftMouseButton`
  (params (Key :type "Key Structure"))
  (bind _springarmcomp (`self.SpringArmComp`))
  (:`Pressed`
    (if (`self.jacking`)
      (bind _asplayer_controller (cast `PlayerController` (`self.GetController`)))
      (bind (_bblockinghit _binitialoverlap _time _distance _location _impactpoint _normal _impactnormal _physmat _hitactor) (`GameplayStatics.BreakHitResult` (`PlayerController.GetHitResultUnderCursorForObjects` _asplayer_controller (`|MakeArray` "ObjectTypeQuery3" "ObjectTypeQuery3" :!type "EObjectTypeQuery Enum") true)))
      (bind _asenemy (cast `/Game/enemies/Enemy` _hitactor)
        (:`then`
          (`KismetSystemLibrary.PrintString` "e")
          (bind (_direction _newtrack_0) (`Timeline|Timeline_0` :!via `PlayFromStart`)
            (:`Update`
              (bind (_returnvalue_x _returnvalue_y _returnvalue_z) (`KismetMathLibrary.BreakVector` (`KismetMathLibrary.VInterpTo` (0.0 -90.0 0.0) (0.0 0.0 0.0) _newtrack_0 1.0)))
              (`Controller.SetControlRotation` (`self.GetController`) (`KismetMathLibrary.MakeRotator` _returnvalue_x _returnvalue_y _returnvalue_z))
              (set `SpringArmComponent.TargetArmLength` (`|EaseFunction` "Linear" _newtrack_0 (`SpringArmComponent.TargetArmLength` _springarmcomp) 400.0) _springarmcomp))
            (:`Finished`
              (bind _asplayer_controller_2 (cast `PlayerController` (`self.GetController`)))
              (set `PlayerController.bShowMouseCursor` false _asplayer_controller_2)
              (set `self.jacking` false)
              (`/Game/enemies/Enemy.pulse` _asenemy))))
        (:`CastFailed`
          (`KismetSystemLibrary.PrintString` (`KismetSystemLibrary.GetDisplayName` _hitactor)))))))

(fn `UserConstructionScript`)