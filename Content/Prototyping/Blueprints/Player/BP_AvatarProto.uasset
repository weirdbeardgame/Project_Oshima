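; BP_AvatarProto is a prototype player character with movement, turning, crouch, sprint and a backstep dodge.
; Custom input events drive movement along the capsule's forward vector and yaw the capsule by a turn rate, with debug prints.
; Sprint changes walk speed and turn rate, while backstep launches the character backward behind a DoOnce that resets after a short delay.
; BeginPlay caches a BP_ControlWireless reference, unused in these graphs.
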(event `self.ReceiveBeginPlay`
  (bind _returnvalue (`GameplayStatics.GetActorOfClass` "/Game/Prototyping/Blueprints/Player/BP_ControlWireless.BP_ControlWireless_C"))
  (set `self.Control` _returnvalue))

(event `Input_Move`
  (params (Value :type "Float (double-precision)"))
  (`self.AddMovementInput` (`SceneComponent.GetForwardVector` (`self.CapsuleComponent`)) Value)
  (`KismetSystemLibrary.PrintString` "Avatar - Move Input Detected"))

(event `Input_Turn`
  (params (Value :type "Float (double-precision)"))
  (`SceneComponent.K2_AddRelativeRotation` (`self.CapsuleComponent`) (`KismetMathLibrary.MakeRotator` 0.0 0.0 (* Value (`self.TurnRate`))) false false)
  (`KismetSystemLibrary.PrintString` "Avatar - Turn Input Detected"))

(event `Input_Crouch`
  ;[1 1 1] Crouching
  (if (`self.Crouched`)
    (`self.UnCrouch`)
    (if (`NavMovementComponent.IsCrouching` (`self.CharacterMovement`))
      (`KismetSystemLibrary.PrintString` "Avatar - Could not Uncrouch!")
      (else
        (set `self.Crouched` false)
        (`KismetSystemLibrary.PrintString` "Avatar - Uncrouched")))
    (elif (`self.CanCrouch`)
      (`self.Crouch`)
      (set `self.Crouched` true)
      (`KismetSystemLibrary.PrintString` "Avatar - Crouched"))))

(event `Input_SprintStart`
  ;[1 1 1] Sprinting
  (set `CharacterMovementComponent.MaxWalkSpeed` 400.0 (`self.CharacterMovement`))
  (set `self.TurnRate` 4.0))

(event `Input_SprintEnd`
  (bind _charactermovement (`self.CharacterMovement`))
  ;[1 1 1] Sprinting
  (set `CharacterMovementComponent.MaxWalkSpeed` 200.0 _charactermovement)
  (set `CharacterMovementComponent.MaxWalkSpeedCrouched` 100.0 _charactermovement)
  (set `self.TurnRate` 2.0))

(event `Input_Backstep`
  (bind (_returnvalue_x _returnvalue_y) (`KismetMathLibrary.BreakVector` (`SceneComponent.GetForwardVector` (`self.CapsuleComponent`))))
  (`/Engine/EditorBlueprintResources/StandardMacros.DoOnce` false :!label _label
    (:`Completed`
      (`self.LaunchCharacter` (`KismetMathLibrary.MakeVector` (* _returnvalue_x -1000.0) (* _returnvalue_y -1000.0)) true)
      (`KismetSystemLibrary.Delay` 0.7)
      (goto _label :!via `Reset`))))

(fn `UserConstructionScript`)