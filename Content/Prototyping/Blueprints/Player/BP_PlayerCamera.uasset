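; Player camera actor that follows the BP_AvatarProto avatar and takes over the player's view with a blend on BeginPlay.
; Each tick it eases its root toward the avatar's location, using delta time as the ease alpha.
; Look input yaws the actor and pitches its spring arm within clamped limits.
; In OverShoulder mode look input is ignored and the actor copies the avatar's yaw instead.
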(event `self.ReceiveBeginPlay`
  (bind _returnvalue (`GameplayStatics.GetActorOfClass` "/Game/Prototyping/Blueprints/Player/BP_AvatarProto.BP_AvatarProto_C"))
  (set `self.Avatar` _returnvalue)
  (`PlayerController.SetViewTargetWithBlend` (`GameplayStatics.GetPlayerController` 0) self 0.5 "VTBlend_Cubic" 0.0 false))

(event `self.ReceiveTick`
  (params (DeltaSeconds :type "Float (single-precision)"))
  (set `self.Delta Seconds` DeltaSeconds)
  (`self.FollowPlayer`)
  (if (`self.OverShoulder`)
    (`self.K2_SetActorRotation` (`KismetMathLibrary.MakeRotator` 0.0 0.0 (.yaw (`self.K2_GetActorRotation` (`self.Avatar`)))))))

(event `FollowPlayer`
  (`SceneComponent.K2_SetWorldLocation` (`self.DefaultSceneRoot`) (`|EaseFunction` "EaseIn" (`self.Delta Seconds`) (`self.K2_GetActorLocation`) (`self.K2_GetActorLocation` (`self.Avatar`)) 0.5) false false))

(event `Input_Look`
  (params (`Value X` :type "Float (double-precision)") (`Value Y` :type "Float (double-precision)"))
  (if (not (`self.OverShoulder`))
    (set `self.RightAxis` `Value X`)
    (set `self.ForwardAxis` `Value Y`)
    (`self.RightInput`)
    (`self.ForwardInput`)))

(event `RightInput`
  (`self.K2_AddActorLocalRotation` (`KismetMathLibrary.MakeRotator` 0.0 0.0 (* (`self.RightAxis`) (* 2.5 1.0)))))

(event `ForwardInput`
  (bind _springarm (`self.SpringArm`))
  (bind (_returnvalue_roll _returnvalue_pitch) (`KismetMathLibrary.BreakRotator` (`SceneComponent.K2_GetComponentRotation` _springarm)))
  (`SceneComponent.K2_AddRelativeRotation` _springarm (`KismetMathLibrary.MakeRotator` 0.0 (* (* (`self.ForwardAxis`) -1.0) (* 2.5 1.0))) false false)
  (`SceneComponent.K2_SetRelativeRotation` _springarm (`KismetMathLibrary.MakeRotator` 0.0 (`KismetMathLibrary.ClampAngle` _returnvalue_pitch -60.0 45.0)) false false))

(fn `UserConstructionScript`)