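; BP_ControlWireless is a possessed input relay that steers the prototype avatar and player camera, which are separate actors.
; On BeginPlay it adds the IMC_Prototype Enhanced Input context and finds both actors by class.
; Move, backstep, sprint, crouch and turn inputs forward to the avatar, while look input goes to the camera.
; Turn input is smoothed by nested easing driven by hold time and frame delta.
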(event `self.ReceiveTick`
  (params (DeltaSeconds :type "Float (single-precision)"))
  (set `self.Delta Seconds` DeltaSeconds))

(event `self.ReceiveBeginPlay`
  (bind _returnvalue (`GameplayStatics.GetPlayerController` 0))
  ;[1 1 1] Adding Input
  (bind _asplayer_controller (cast `PlayerController` (`self.GetController`)))
  (`WidgetBlueprintLibrary.SetInputMode_GameOnly` _returnvalue)
  (bind _returnvalue_2 (pcsubsystem `EnhancedInputLocalPlayerSubsystem` _asplayer_controller))
  (`/Engine/EditorBlueprintResources/StandardMacros.IsValid` _returnvalue_2
    (:`Is Valid`
      (`EnhancedInputSubsystemInterface.AddMappingContext` _returnvalue_2 "/Game/Prototyping/Blueprints/Input/IMC_Prototype.IMC_Prototype" 0 (struct))
      (`self.EnableInput` _returnvalue)
      (bind _returnvalue_3 (`GameplayStatics.GetActorOfClass` "/Game/Prototyping/Blueprints/Player/BP_AvatarProto.BP_AvatarProto_C"))
      (`/Engine/EditorBlueprintResources/StandardMacros.IsValid` _returnvalue_3
        (:`Is Valid`
          (set `self.Avatar` _returnvalue_3)
          (bind _returnvalue_4 (`GameplayStatics.GetActorOfClass` "/Game/Prototyping/Blueprints/Player/BP_PlayerCamera.BP_PlayerCamera_C"))
          (`/Engine/EditorBlueprintResources/StandardMacros.IsValid` _returnvalue_4
            (:`Is Valid`
              (set `self.Camera` _returnvalue_4))))))))

(event `EnhancedInput|/Game/Prototyping/Blueprints/Input/IA_Backstep`
  (params (ActionValue :type Boolean) (ElapsedSeconds :type "Float (double-precision)") (TriggeredSeconds :type "Float (double-precision)") (InputAction :type "InputAction Object Reference" :default "/Game/Prototyping/Blueprints/Input/IA_Backstep.IA_Backstep"))
  (:`Completed`
    (`/Game/Prototyping/Blueprints/Player/BP_AvatarProto.Input_Backstep` (`self.Avatar`) :!label _label)))

(event `EnhancedInput|/Game/Prototyping/Blueprints/Input/IA_Forward`
  (params (ActionValue :type Boolean) (ElapsedSeconds :type "Float (double-precision)") (TriggeredSeconds :type "Float (double-precision)") (InputAction :type "InputAction Object Reference" :default "/Game/Prototyping/Blueprints/Input/IA_Forward.IA_Forward"))
  (:`Triggered`
    (`/Game/Prototyping/Blueprints/Player/BP_AvatarProto.Input_Move` (`self.Avatar`) 1.0)))

(event `EnhancedInput|/Game/Prototyping/Blueprints/Input/IA_Backward`
  (params (ActionValue :type Boolean) (ElapsedSeconds :type "Float (double-precision)") (TriggeredSeconds :type "Float (double-precision)") (InputAction :type "InputAction Object Reference" :default "/Game/Prototyping/Blueprints/Input/IA_Backward.IA_Backward"))
  (:`Started`
    (goto _label)))

(event `EnhancedInput|/Game/Prototyping/Blueprints/Input/IA_Thrust`
  (params (ActionValue :type "Float (double-precision)") (ElapsedSeconds :type "Float (double-precision)") (TriggeredSeconds :type "Float (double-precision)") (InputAction :type "InputAction Object Reference" :default "/Game/Prototyping/Blueprints/Input/IA_Thrust.IA_Thrust"))
  (:`Triggered`
    (bind _output_get (set `self.MoveValue` ActionValue))
    (`/Game/Prototyping/Blueprints/Player/BP_AvatarProto.Input_Move` (`self.Avatar`) _output_get))
  (:`Started`
    (`KismetSystemLibrary.PrintString` "Controller - Move Input Detected")))

(event `Key|Q`
  (params (Key :type "Key Structure"))
  (:`Pressed`
    (`KismetSystemLibrary.PrintString` "Controller - Q Pressed")))

(event `EnhancedInput|/Game/Prototyping/Blueprints/Input/IA_Turn`
  (params (ActionValue :type "Float (double-precision)") (ElapsedSeconds :type "Float (double-precision)") (TriggeredSeconds :type "Float (double-precision)") (InputAction :type "InputAction Object Reference" :default "/Game/Prototyping/Blueprints/Input/IA_Turn.IA_Turn"))
  (:`Triggered`
    (`/Game/Prototyping/Blueprints/Player/BP_AvatarProto.Input_Turn` (`self.Avatar`) (`|EaseFunction` "EaseIn" (`self.Delta Seconds`) (`self.TurnEased`) (`KismetMathLibrary.FInterpEaseInOut` 0.0 ActionValue (`KismetMathLibrary.FClamp` TriggeredSeconds) 0.2) 0.3))))

(event `EnhancedInput|/Game/Prototyping/Blueprints/Input/IA_Sprint`
  (params (ActionValue :type Boolean) (ElapsedSeconds :type "Float (double-precision)") (TriggeredSeconds :type "Float (double-precision)") (InputAction :type "InputAction Object Reference" :default "/Game/Prototyping/Blueprints/Input/IA_Sprint.IA_Sprint"))
  (bind _avatar (`self.Avatar`))
  (:`Started`
    (`/Game/Prototyping/Blueprints/Player/BP_AvatarProto.Input_SprintStart` _avatar)
    (`KismetSystemLibrary.PrintString` "Controller - Sprint has been triggered!"))
  (:`Completed`
    (`/Game/Prototyping/Blueprints/Player/BP_AvatarProto.Input_SprintEnd` _avatar)))

(event `EnhancedInput|/Game/Prototyping/Blueprints/Input/IA_Crouch`
  (params (ActionValue :type Boolean) (ElapsedSeconds :type "Float (double-precision)") (TriggeredSeconds :type "Float (double-precision)") (InputAction :type "InputAction Object Reference" :default "/Game/Prototyping/Blueprints/Input/IA_Crouch.IA_Crouch"))
  (:`Started`
    (`/Game/Prototyping/Blueprints/Player/BP_AvatarProto.Input_Crouch` (`self.Avatar`))))

(event `EnhancedInput|/Game/Prototyping/Blueprints/Input/IA_Interact`
  (params (ActionValue :type Boolean) (ElapsedSeconds :type "Float (double-precision)") (TriggeredSeconds :type "Float (double-precision)") (InputAction :type "InputAction Object Reference" :default "/Game/Prototyping/Blueprints/Input/IA_Interact.IA_Interact")))

(event `EnhancedInput|/Game/Input/IA_Look`
  (params (ActionValue :type "Vector2D Structure") (ElapsedSeconds :type "Float (double-precision)") (TriggeredSeconds :type "Float (double-precision)") (InputAction :type "InputAction Object Reference" :default "/Game/Input/IA_Look.IA_Look"))
  (:`Triggered`
    (`/Game/Prototyping/Blueprints/Player/BP_PlayerCamera.Input_Look` (`self.Camera`) ActionValue_X ActionValue_Y)))

(fn `UserConstructionScript`)